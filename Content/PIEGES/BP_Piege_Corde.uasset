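; Rope trap actor that kills enemies it strikes once released.
; LaunchTrap enables physics on the Cylinder component to set the trap in motion.
; When the Box hits a living Ennemy, it calls Death with a strong impulse along the Box's velocity.
; The hit also spawns a half-scale explosion effect at the Box and plays a gunshot sound at the world origin.
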(event OnComponentHit(Box)
  (params (HitComponent :type Primitive%20Component%20Object%20Reference) (OtherActor :type Actor%20Object%20Reference) (OtherComp :type Primitive%20Component%20Object%20Reference) (NormalImpulse :type Vector :default "0, 0, 0") (Hit :type Hit%20Result%20Structure%20%28by%20ref%29))
  (bind _asennemy (Utilities|Casting|CastToEnnemy OtherActor))
  (if (not (Default|IsDead _asennemy))
    (Default|Death _asennemy (* (Math|Vector|Normalize (Transformation|GetComponentVelocity (Variables|Default|GetBox))) 1.25e+04) "None")
    (Effects|SpawnEmitteratLocation "/Game/MilitaryWeapSilver/FX/P_Grenade_Explosion_01.P_Grenade_Explosion_01" (Transformation|GetWorldLocation (Variables|Default|GetBox)) "0, 0, 0" "0.500000,0.500000,0.500000" true "AutoRelease")
    (Audio|PlaySoundatLocation "/Game/MilitaryWeapSilver/Sound/Pistol/Wavs/PistolA_Fire04.PistolA_Fire04" "0, 0, 0" "0, 0, 0" 1.0 1.0 0.0 0 0 0)))

(event EventBeginPlay
  (|CallParentFunction) ; This node is disabled and will not be called.\nDrag off pins to build functionality.
)

(event Collision|EventActorBeginOverlap
  (params (OtherActor :type Actor%20Object%20Reference))
  (|CallParentFunction OtherActor) ; This node is disabled and will not be called.\nDrag off pins to build functionality.
)

(event EventTick
  (params (DeltaSeconds :type Float%20%28single-precision%29))
  (|CallParentFunction DeltaSeconds) ; This node is disabled and will not be called.\nDrag off pins to build functionality.
)

(event EventLaunchTrap
  (Physics|SetSimulatePhysics (Variables|Default|GetCylinder) true))

(fn ConstructionScript
  (|CallParentFunction))