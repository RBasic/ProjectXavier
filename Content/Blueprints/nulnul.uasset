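; A VR motion controller hand Blueprint, apparently a scratch copy, whose only logic is an action that either fires a pistol or grabs, with no event triggering it.
; With the pistol mesh in hand, it checks the HUD_Bullet widget's ammo, then spawns a tracer at the laser origin and decrements the count, or plays a sound when empty.
; Otherwise it picks up the nearby actor through PickupMessage and rumbles the controller.
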(fn ConstructionScript)