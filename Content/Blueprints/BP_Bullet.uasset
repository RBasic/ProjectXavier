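; BP_Bullet is a projectile that spawns almost frozen in time, follows a trajectory of points and kills enemies it hits.
; A near-zero custom time dilation holds it until StopSlowmotion restores normal speed.
; The bttr event replays a timeline per segment, sweeping the capsule between TrajBullet points and orienting it along the path.
; Overlapping an Ennemy's skeletal mesh calls Death with the hit bone and an impulse from the impact normal.
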(event OnComponentBeginOverlap(Capsule)
  (params (OverlappedComponent :type Primitive%20Component%20Object%20Reference) (OtherActor :type Actor%20Object%20Reference) (OtherComp :type Primitive%20Component%20Object%20Reference) (OtherBodyIndex :type Integer) (bFromSweep :type Boolean) (SweepResult :type Hit%20Result%20Structure%20%28by%20ref%29))
  (bind _asennemy (Utilities|Casting|CastToEnnemy OtherActor))
  (Utilities|Casting|CastToSkeletalMeshComponent OtherComp)
  (Default|Death _asennemy (* (.impactnormal SweepResult) -3e+03) (.hitbonename SweepResult)))

(event Custom|bttr
  (bind _trajbullet (Variables|Default|GetTrajBullet))
  (bind _capsule (Variables|Default|GetCapsule))
  (bind _bulletindex (Variables|Default|GetBulletIndex))
  (bind _bulletindex_2 (Variables|Default|GetBulletIndex))
  (bind _returnvalue (+ _bulletindex 1))
  (bind _output (Utilities|Array|Get(acopy) _trajbullet _bulletindex))
  (bind _output_2 (Utilities|Array|Get(acopy) _trajbullet _returnvalue))
  (bind _returnvalue_2 (Math|Rotator|FindLookatRotation _output _output_2))
  (bind _newtrack_0 (Timeline|Timeline_0 PlayFromStart)
    (:Update
      (Transformation|SetWorldLocation _capsule (Math|Vector|Lerp(Vector) _output _output_2 _newtrack_0) true false)
      (Transformation|SetWorldRotation _capsule (Math|Rotator|MakeRotator (.roll _returnvalue_2) (+ (.pitch _returnvalue_2) 9e+01) (.yaw _returnvalue_2)) false false))
    (:Finished
      (Math|Integer|IncrementInt _bulletindex_2
        (:%20%20
          (if (not (>= _bulletindex_2 (Utilities|Array|LastIndex _trajbullet)))
            (Timeline|Timeline_0 PlayFromStart)))))))

(event Custom|StopSlowmotion
  (Variables|Default|SetCustomTimeDilation 1.0))

(event EventBeginPlay
  (Variables|Default|SetCustomTimeDilation 1e-06))

(fn ConstructionScript)