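; Enemy character for a motion-controller (VR) game that chases the player pawn and ragdolls when killed.
; It starts nearly frozen through CustomTimeDilation until StartMoving restores normal time and issues AIMoveTo toward the player.
; Death runs once, enabling mesh physics with a bone impulse, disabling capsule collision, and playing an explosion effect and a gunshot sound.
; Capsule overlap with BP_MotionController only prints "Fail", and the pawn cast on Tick feeds only an unconnected move node.
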(event OnComponentBeginOverlap(CapsuleComponent)
  (params (OverlappedComponent :type Primitive%20Component%20Object%20Reference) (OtherActor :type Actor%20Object%20Reference) (OtherComp :type Primitive%20Component%20Object%20Reference) (OtherBodyIndex :type Integer) (bFromSweep :type Boolean) (SweepResult :type Hit%20Result%20Structure%20%28by%20ref%29))
  (Utilities|Casting|CastToBP_MotionController OtherActor)
  (Development|PrintString "Fail"))

(event Custom|Death
  (params (Impulse :type Vector) (BoneName :type Name))
  (bind _mesh (Variables|Character|GetMesh))
  (Utilities|FlowControl|DoOnce false
    (:Completed
      (Physics|SetSimulatePhysics _mesh true)
      (Collision|SetCollisionProfileName _mesh "Ragdoll" :!class /Script/Engine.PrimitiveComponent)
      (Physics|AddImpulse (Variables|Character|GetMesh) Impulse BoneName true)
      (Effects|SpawnEmitteratLocation "/Game/MilitaryWeapSilver/FX/P_Grenade_Explosion_01.P_Grenade_Explosion_01" (Transformation|GetActorLocation) "0, 0, 0" "0.200000,0.200000,0.200000" true "AutoRelease")
      (Audio|PlaySoundatLocation "/Game/MilitaryWeapSilver/Sound/Pistol/Wavs/PistolA_Fire04.PistolA_Fire04" "0, 0, 0" "0, 0, 0" 1.0 1.0 0.0 0 0 0)
      (Collision|SetCollisionProfileName (Variables|Collision|GetCapsuleComponent) "NoCollision" :!class /Script/Engine.PrimitiveComponent))))

(event Custom|StartMoving
  (Variables|Default|SetCustomTimeDilation 1.0)
  (AI|AIMoveTo self "0, 0, 0" (Game|Player|GetPlayerPawn 0) 5.0 false))

(event EventTick
  (params (DeltaSeconds :type Float%20%28single-precision%29))
  (Utilities|FlowControl|Sequence
    (:then_0
      (bind _asmotion_controller_pawn (Utilities|Casting|CastToMotionControllerPawn (Game|Player|GetPlayerPawn 0))))))

(event EventBeginPlay
  (Variables|Default|SetCustomTimeDilation 1e-06))

(fn ConstructionScript)