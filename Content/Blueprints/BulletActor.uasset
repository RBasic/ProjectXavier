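; BulletActor is an actor that moves its particle system along a precomputed bullet trajectory stored in the TrajBullet point array.
; The bttr event starts a timeline that interpolates the particle's world location between the current point and the next, without sweeping.
; Each finished timeline increments BulletIndex and replays for the following segment until the last point is reached.
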(event Custom|bttr
  (bind _trajbullet (Variables|Default|GetTrajBullet))
  (bind _bulletindex (Variables|Default|GetBulletIndex))
  (bind _bulletindex_2 (Variables|Default|GetBulletIndex))
  (bind _newtrack_0 (Timeline|Timeline_0 PlayFromStart)
    (:Update
      (Transformation|SetWorldLocation (Variables|Default|GetParticleSystem) (Math|Vector|Lerp(Vector) (Utilities|Array|Get(acopy) _trajbullet _bulletindex) (Utilities|Array|Get(acopy) _trajbullet (+ _bulletindex 1)) _newtrack_0) false false))
    (:Finished
      (Math|Integer|IncrementInt _bulletindex_2
        (:%20%20
          (if (not (>= _bulletindex_2 (Utilities|Array|LastIndex _trajbullet)))
            (Timeline|Timeline_0 PlayFromStart)))))))

(fn ConstructionScript)